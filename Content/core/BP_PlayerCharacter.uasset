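; BP_PlayerCharacter is the on-foot player character, which can walk, look around and get into a car.
; It adds an Enhanced Input mapping context on BeginPlay for movement along actor axes and mouse look scaled by sensitivity and delta time.
; Interact runs a stationary, debug-drawn box trace just ahead for Pawn objects.
; On hitting a BP_Car, the player controller possesses the car and the character destroys itself.
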(event `self.ReceiveBeginPlay`
  (`EnhancedInputSubsystemInterface.AddMappingContext` (pcsubsystem `EnhancedInputLocalPlayerSubsystem` (`GameplayStatics.GetPlayerController` 0)) "/Game/core/IMC_Controls.IMC_Controls" 0 (struct)))

(event `EnhancedInput|/Game/core/IA_Movement`
  (params (ActionValue :type "Vector2D Structure") (ElapsedSeconds :type "Float (double-precision)") (TriggeredSeconds :type "Float (double-precision)") (InputAction :type "InputAction Object Reference" :default "/Game/core/IA_Movement.IA_Movement"))
  (bind (_x _y) (`KismetMathLibrary.BreakVector2D` ActionValue))
  (:`Triggered`
    (`self.AddMovementInput` (`self.GetActorForwardVector`) _y)
    (`self.AddMovementInput` (`self.GetActorRightVector`) _x)))

(event `EnhancedInput|/Game/core/IA_Mouse`
  (params (ActionValue :type "Vector2D Structure") (ElapsedSeconds :type "Float (double-precision)") (TriggeredSeconds :type "Float (double-precision)") (InputAction :type "InputAction Object Reference" :default "/Game/core/IA_Mouse.IA_Mouse"))
  (bind (_x _y) (`KismetMathLibrary.BreakVector2D` ActionValue))
  (:`Triggered`
    (`self.AddControllerYawInput` (* _x (`GameplayStatics.GetWorldDeltaSeconds`) (`self.MouseSens`)))
    (`self.AddControllerPitchInput` (* _y (`GameplayStatics.GetWorldDeltaSeconds`) (`self.MouseSens`)))))

(event `EnhancedInput|/Game/core/IA_Interact`
  (params (ActionValue :type Boolean) (ElapsedSeconds :type "Float (double-precision)") (TriggeredSeconds :type "Float (double-precision)") (InputAction :type "InputAction Object Reference" :default "/Game/core/IA_Interact.IA_Interact"))
  (bind _returnvalue (`self.GetActorForwardVector`))
  (bind _returnvalue_2 (+ (`self.K2_GetActorLocation`) (* _returnvalue 30.0)))
  (:`Started`
    (bind (_outhit _returnvalue_3) (`KismetSystemLibrary.BoxTraceSingleForObjects` :`Start` _returnvalue_2 :`End` _returnvalue_2 :`HalfSize` (110.0 111.0 110.0) :`Orientation` (`KismetMathLibrary.Conv_VectorToRotator` _returnvalue) :`ObjectTypes` (`|MakeArray` "ObjectTypeQuery3" :!type "EObjectTypeQuery Enum") :`DrawDebugType` "ForDuration"))
    (if _returnvalue_3
      (if _returnvalue_3
        (bind _asbp_car (cast `/Game/core/BP_Car` (`.HitActor` (`GameplayStatics.BreakHitResult` _outhit))))
        (`Controller.UnPossess` (`GameplayStatics.GetPlayerController` 0))
        (`Controller.Possess` (`GameplayStatics.GetPlayerController` 0) _asbp_car)
        (`self.K2_DestroyActor`)))))

(fn `UserConstructionScript`)