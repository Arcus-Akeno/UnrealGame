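; Offensive vehicle Blueprint with a player-aimed turret that fires projectiles.
; Mouse input yaws the turret at TurretSpeed, and the shoot input spawns ProjectileToShoot at ShootPosition using the turret's rotation, with a debug "Bang" print.
; Firing requires zero Cooldown, but the limit is unfinished: GoOnCooldown is empty, ReduceCooldown zeroes Cooldown every tick, and its clamped countdown is unconnected.
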(event `self.ReceiveBeginPlay`
  (`parent.ReceiveBeginPlay`))

(event `self.ReceiveTick`
  (params (DeltaSeconds :type "Float (single-precision)"))
  (`parent.ReceiveTick` DeltaSeconds)
  (`self.ReduceCooldown`))

(event `Shoot`
  (bind _offcooldown (`self.CanShoot`))
  (if _offcooldown
    (`|SpawnActorFromClass` (`self.ProjectileToShoot`) (`KismetMathLibrary.MakeTransform` (`SceneComponent.K2_GetComponentLocation` (`self.ShootPosition`)) (`SceneComponent.K2_GetComponentRotation` (`self.Turret`))) "Undefined" "MultiplyWithRoot" null null)
    (`KismetSystemLibrary.PrintString` "Bang" true true (struct :`G` 0.66 :`B` 1.0 :`A` 1.0) 20.0)
    (`self.GoOnCooldown`)))

(event `EnhancedInput|/Game/core/IA_Mouse`
  (params (ActionValue :type "Vector2D Structure") (ElapsedSeconds :type "Float (double-precision)") (TriggeredSeconds :type "Float (double-precision)") (InputAction :type "InputAction Object Reference" :default "/Game/core/IA_Mouse.IA_Mouse"))
  (:`Triggered`
    (`SceneComponent.K2_AddLocalRotation` (`self.Turret`) (`KismetMathLibrary.MakeRotator` 0.0 0.0 (* (`KismetMathLibrary.BreakVector2D` ActionValue) (`GameplayStatics.GetWorldDeltaSeconds`) (`self.TurretSpeed`) -1.0)) false false)))

(event `EnhancedInput|/Game/core/IA_Shoot`
  (params (ActionValue :type Boolean) (ElapsedSeconds :type "Float (double-precision)") (TriggeredSeconds :type "Float (double-precision)") (InputAction :type "InputAction Object Reference" :default "/Game/core/IA_Shoot.IA_Shoot"))
  (:`Started`
    (`self.Shoot`)))

(fn `CanShoot`
  (returns (offcooldown :type Boolean))
  (return (== (`self.Cooldown`) 0.0)))

(fn `GoOnCooldown`)

(fn `ReduceCooldown`
  (set `self.Cooldown` 0.0))

(fn `UserConstructionScript`
  (`parent.UserConstructionScript`))