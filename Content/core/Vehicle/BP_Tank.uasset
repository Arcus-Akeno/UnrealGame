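; BP_Tank is a tank vehicle Blueprint that tracks a team colour according to the controller possessing it.
; Possession passes BP_PC's TeamColor to ChangeTeamColour, and unpossession passes white.
; That event stores the colour, then recreates a dynamic M_TeamColour instance on the Cube's second material slot, as BeginPlay also does.
; No node here writes the colour into the material.
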(event `ChangeTeamColour`
  (params (LinearColour :type "LinearColor Structure"))
  (set `self.Linear Colour` LinearColour)
  (bind _returnvalue (`PrimitiveComponent.CreateDynamicMaterialInstance` (`self.Cube`) 1 "/Game/core/Art/3D/M_TeamColour.M_TeamColour" "None" :!label _label))
  (set `self.TeamColour` _returnvalue))

(event `self.ReceiveBeginPlay`
  (`parent.ReceiveBeginPlay`)
  (goto _label))

(event `self.ReceivePossessed`
  (params (NewController :type "Controller Object Reference"))
  (bind _asbp_pc (cast `/Game/core/BP_PC` NewController))
  (`self.ChangeTeamColour` (`/Game/core/BP_PC.TeamColor` _asbp_pc)))

(event `self.ReceiveUnpossessed`
  (params (OldController :type "Controller Object Reference"))
  (`self.ChangeTeamColour` (struct :`R` 1.0 :`G` 1.0 :`B` 1.0 :`A` 1.0)))

(fn `UserConstructionScript`
  (`parent.UserConstructionScript`))