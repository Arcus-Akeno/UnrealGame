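; BP_Tank is a tank Blueprint whose turret turns with mouse input.
; The input_Tank graph handles the IA_Mouse Enhanced Input action, adding local yaw to the Cylinder component from the X axis value, negated and scaled by TurretSpeed and frame delta time.
; The event graph holds only disabled default events, and the construction script just calls its parent.
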(event `EnhancedInput|/Game/core/IA_Mouse`
  (params (ActionValue :type "Vector2D Structure") (ElapsedSeconds :type "Float (double-precision)") (TriggeredSeconds :type "Float (double-precision)") (InputAction :type "InputAction Object Reference" :default "/Game/core/IA_Mouse.IA_Mouse"))
  (:`Triggered`
    (`SceneComponent.K2_AddLocalRotation` (`self.Cylinder`) (`KismetMathLibrary.MakeRotator` 0.0 0.0 (* (`KismetMathLibrary.BreakVector2D` ActionValue) (`GameplayStatics.GetWorldDeltaSeconds`) (`self.TurretSpeed`) -1.0)) false false)))

(fn `UserConstructionScript`
  (`parent.UserConstructionScript`))